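; Player pawn for a grid-based tabletop with a top-down drag-and-zoom camera, token handling and toggleable GM widgets.
; Left-click traces pick up tagged actors, which follow the cursor each tick until dropped; E destroys the held one.
; TruncateLocation snaps drops to grid lines for "Large" tokens and cell centers for others.
; Right-drag pans, the wheel shifts capsule height, and panning copies player 0's pawn location onto player 1's.
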(event Custom|Movement
  ;[1 1 1] Drag Camera Functionality
  (bind _returnvalue (Class|WidgetLayoutLibrary|GetMousePositiononViewport))
  (Variables|Default|SetPreviousTouchLocation _returnvalue))

(event Custom|Cam%20Movement
  (bind _returnvalue (Game|GetPlayerController 0))
  (bind _heldtoken (Variables|Default|GetHeldToken))
  (bind (_worldlocation _worlddirection) (Game|Player|ConvertMouseLocationToWorldSpace _returnvalue))
  ;[1 1 1] Move Clicked Token
  (if (Utilities|IsValid _heldtoken)
    (bind _outactors (Actor|GetAllActorswithTag "Token"))
    (bind _outhit (Collision|LineTraceByChannel _worldlocation (+ _worldlocation (* _worlddirection 1e+04)) "TraceTypeQuery1" false _outactors "None"))
    (Transformation|SetActorLocation _heldtoken (.location _outhit) false false))
  ;[1 1 1] Drag Camera Functionality
  (if (Game|Player|IsInputKeyDown (Game|GetPlayerController 0) "RightMouseButton")
    (bind _returnvalue_2 (Class|WidgetLayoutLibrary|GetMousePositiononViewport))
    (Variables|Default|SetNewTouchLocation _returnvalue_2)
    (Transformation|AddActorWorldOffset (Math|Vector|MakeVector (.x (- (Variables|Default|GetNewTouchLocation) (Variables|Default|GetPreviousTouchLocation))) (.y (- (Variables|Default|GetNewTouchLocation) (Variables|Default|GetPreviousTouchLocation))) 0.0))
    (Variables|Default|SetPreviousTouchLocation (Variables|Default|GetNewTouchLocation))
    (CallFunction|ClientMovement)))

(event Custom|Client%20Movement
  (bind _returnvalue (Game|GetPlayerState 0))
  (bind _returnvalue_2 (PlayerState|GetPawn _returnvalue))
  (bind _returnvalue_3 (Transformation|GetActorLocation _returnvalue_2))
  ;[1 1 1] Drag Camera Functionality
  (Transformation|SetActorLocation (PlayerState|GetPawn (Game|GetPlayerState 1)) _returnvalue_3 false false)
  (Development|PrintString (Utilities|String|ToString(Vector) _returnvalue_3) true true "(R=1.000000,G=0.000000,B=0.109532,A=1.000000)"))

(event EventBeginPlay
  ;[1 1 1] Create GM HUD
  (bind _returnvalue (UserInterface|CreateWidget "/Game/Blueprints/Widgets/W_GMHUD.W_GMHUD_C"))
  (Variables|Default|SetHUDRef _returnvalue))

(event EventTick
  (params (DeltaSeconds :type Float%20%28single-precision%29))
  ;[1 1 1] Move Clicked Token
  (CallFunction|CamMovement))

(event Input|MouseEvents|MouseWheelAxis
  (params (AxisValue :type Float%20%28single-precision%29))
  (bind _capsulecomponent (Variables|Collision|GetCapsuleComponent))
  (bind _relativelocation (Variables|/Script/Engine.SceneComponent|GetRelativeLocation _capsulecomponent))
  ;[1 1 1] Zoom Camera
  (if (!= AxisValue 0.0)
    (Transformation|SetRelativeLocation _capsulecomponent (Math|Vector|MakeVector (.x _relativelocation) (.y _relativelocation) (+ (.z _relativelocation) (* AxisValue 1e+02))) false false)))

(event Input|MouseEvents|LeftMouseButton
  (params (Key :type Key%20Structure :default "None"))
  (bind _returnvalue (Game|GetPlayerController 0))
  (bind (_worldlocation _worlddirection) (Game|Player|ConvertMouseLocationToWorldSpace _returnvalue))
  ;[1 1 1] Trace directly to mouse location
  (:Pressed
    (if (Utilities|IsValid (Variables|Default|GetHeldToken))
      (bind _gridlocation (CallFunction|TruncateLocation (Transformation|GetActorLocation (Variables|Default|GetHeldToken)) (Variables|Default|GetHeldToken)))
      (Transformation|SetActorLocation (Variables|Default|GetHeldToken) _gridlocation false false)
      (Variables|Default|SetHeldToken 0)
      (else
        (bind _outhit (Collision|LineTraceByChannel _worldlocation (+ _worldlocation (* _worlddirection 1e+04)) "TraceTypeQuery1" false 0 "ForDuration"))
        (Variables|Default|SetDistanceFromToken (.distance _outhit))
        (if (Utilities|Array|IsValidIndex (Variables|/Script/Engine.Actor|GetTags (.hitactor _outhit)))
          (Variables|Default|SetHeldToken (.hitactor _outhit)))))))

(event Input|KeyboardEvents|Q
  (params (Key :type Key%20Structure :default "None"))
  (bind _hudref (Variables|Default|GetHUDRef))
  ;[1 1 1] Spawn HUD Widget
  (:Pressed
    (if (Variables|Default|GetHUDOpened?)
      (Widget|RemovefromParent _hudref)
      (Variables|Default|SetHUDOpened? false)
      (else
        (UserInterface|Viewport|AddtoViewport _hudref 0)
        (Variables|Default|SetHUDOpened? true)))))

(event Input|MouseEvents|RightMouseButton
  (params (Key :type Key%20Structure :default "None"))
  ;[1 1 1] Drag Camera Functionality
  (:Pressed
    (CallFunction|Movement)))

(event Input|KeyboardEvents|E
  (params (Key :type Key%20Structure :default "None"))
  ;[1 1 1] Destroy Held Token
  (:Pressed
    (if (Utilities|IsValid (Variables|Default|GetHeldToken))
      (Actor|DestroyActor (Variables|Default|GetHeldToken))
      (Variables|Default|SetHeldToken 0))))

(event Input|KeyboardEvents|Tab
  (params (Key :type Key%20Structure :default "None"))
  ;[1 1 1] Spawn Logistic Widget
  (:Pressed
    (Utilities|FlowControl|FlipFlop
      (:A
        (bind _returnvalue (UserInterface|CreateWidget "/Game/Blueprints/Widgets/W_ScreenSize.W_ScreenSize_C"))
        (UserInterface|Viewport|AddtoViewport _returnvalue 0))
      (:B
        (Viewport|RemoveAllWidgets)))))

(fn ConstructionScript)

(fn TruncateLocation
  (params (OriginalLocation :type Vector) (HeldToken :type Actor%20Object%20Reference))
  (bind _gridscale (Variables|Default|GetGridScale))
  (bind _gridsize (Variables|Default|GetGridSize))
  (bind _gridsize_2 (Variables|Default|GetGridSize))
  (bind _returnvalue (* OriginalLocation _gridscale))
  (bind _returnvalue_2 (* OriginalLocation _gridscale))
  (bind _returnvalue_3 (Class|KismetMathLibrary|FTruncVector _returnvalue_2))
  (if (Actor|ActorHasTag HeldToken "Large")
    (return (Math|Vector|MakeVector (* _gridsize (Math|Float|Round (.x _returnvalue))) (* (Math|Float|Round (.y _returnvalue)) _gridsize) 1e+01))
    (else
      (return (Math|Vector|MakeVector (+ (* _gridsize_2 (.x _returnvalue_3)) (/ _gridsize_2 2.0)) (+ (* (.y _returnvalue_3) _gridsize_2) (/ _gridsize_2 2.0)) 1e+01)))))