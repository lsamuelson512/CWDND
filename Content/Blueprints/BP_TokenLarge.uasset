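; BP_TokenLarge is a large token with a cylinder mesh whose surface image can be loaded from a URL at runtime.
; Its construction script creates a dynamic instance of the cylinder's material, with MissingTexture as the placeholder Base Color.
; The ChangeMaterial event downloads the image and applies it to that parameter on success, printing status messages for start, finish and failure.
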(event Custom|Change%20Material
  (params (URL :type String))
  (bind _texture (|DownloadImage URL)
    (:then
      (Development|PrintString "Started Downloading"))
    (:OnSuccess
      (Rendering|Material|SetTextureParameterValue (Variables|Default|GetDynamicMaterial) "Base Color" _texture)
      (Development|PrintString "Finished Downloading"))
    (:OnFail
      (Development|PrintString "Failed Downloading"))))

(fn ConstructionScript
  (bind _returnvalue (Rendering|Material|CreateDynamicMaterialInstance (Rendering|Material|GetMaterial (Variables|Default|GetCylinder) 0) "None" "None" :!class /Script/Engine.KismetMaterialLibrary))
  (bind _output_get (Variables|Default|SetDynamicMaterial _returnvalue))
  (Rendering|Material|SetTextureParameterValue _output_get "Base Color" "/Game/Textures/MissingTexture.MissingTexture")
  (Rendering|Material|SetMaterial (Variables|Default|GetCylinder) 0 _output_get))